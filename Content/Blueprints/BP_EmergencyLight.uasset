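; BP_EmergencyLight is an emergency light actor that shows itself with a siren and blinking light in three scripted bursts.
; BeginPlay hides it, then uses chained Delays to reveal it for fixed windows, calling EMERGENCY and stopping the siren after each.
; EMERGENCY starts the siren if silent and sets a looping timer at the Frecuencia interval, which toggles PointLight visibility through ToggleLight and is never cleared.
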(event Custom|EMERGENCY
  (if (not (Audio|Components|Audio|IsPlaying (Variables|Default|GetSiren)))
    (Audio|Components|Audio|Play (Variables|Default|GetSiren) 0.0)
    (Utilities|Time|SetTimerbyFunctionName 0 "ToggleLight" (Variables|Default|Getfrecuencia) true)))

(event EventBeginPlay
  (Rendering|SetActorHiddenInGame true)
  (Utilities|FlowControl|Delay 1.6e+02)
  (Rendering|SetActorHiddenInGame false)
  (CallFunction|EMERGENCY)
  (Utilities|FlowControl|Delay 1e+01)
  (Audio|Components|Audio|Stop (Variables|Default|GetSiren))
  (Rendering|SetActorHiddenInGame true)
  (Utilities|FlowControl|Delay 2e+01)
  (Rendering|SetActorHiddenInGame false)
  (CallFunction|EMERGENCY)
  (Utilities|FlowControl|Delay 1e+01)
  (Audio|Components|Audio|Stop (Variables|Default|GetSiren))
  (Rendering|SetActorHiddenInGame true)
  (Utilities|FlowControl|Delay 1e+01)
  (Rendering|SetActorHiddenInGame false)
  (CallFunction|EMERGENCY)
  (Utilities|FlowControl|Delay 1e+01)
  (Audio|Components|Audio|Stop (Variables|Default|GetSiren))
  (Rendering|SetActorHiddenInGame true))

(event Collision|EventActorBeginOverlap
  (params (OtherActor :type Actor%20Object%20Reference)))

(event EventTick
  (params (DeltaSeconds :type Float%20%28single-precision%29)))

(fn ConstructionScript)

(fn ToggleLight
  (Rendering|ToggleVisibility (Variables|Default|GetPointLight) false))